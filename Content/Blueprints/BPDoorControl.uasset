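; BPDoorControl is a door control that links a button in a JavaScript-driven interface to a target door.
; A button click event calls TriggerDoors on TargetDoor.
; The construction script binds to the door's state-change event.
; The state-change handler creates a NotifyDoorState JavaScript call object, sets the new state and invokes it in the script context, keeping the interface in sync.
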(event `Received_ButtonClicked`
  (`/Game/ExampleContent/Level_Scripting/BP_Double_Doors.Trigger doors` (`self.TargetDoor`)))

(fn `OnDoorStateChanged`
  (params (NewDoorState :type "/Game/Blueprints/EDoorState Enum" :default "NewEnumerator0"))
  (bind _asjscall_door_control_notify_door_state (cast `/Game/Blueprints/JSCall_DoorControl_NotifyDoorState` (`RadiantJavaScriptFunctionCallLibrary.NewJavaScriptFunctionCallInstance` "/Game/Blueprints/JSCall_DoorControl_NotifyDoorState.JSCall_DoorControl_NotifyDoorState_C")))
  (set `/Game/Blueprints/JSCall_DoorControl_NotifyDoorState.DoorState` NewDoorState _asjscall_door_control_notify_door_state)
  (`RadiantJavaScriptFunctionCall.Invoke` _asjscall_door_control_notify_door_state (`self.GetJavaScriptCallContext`)))

(fn `UserConstructionScript`
  (`parent.UserConstructionScript`)
  (add `/Game/ExampleContent/Level_Scripting/BP_Double_Doors.DoorStateChanged` (`self.TargetDoor`) (`|CreateDelegate` self :!event `OnDoorStateChanged`)))